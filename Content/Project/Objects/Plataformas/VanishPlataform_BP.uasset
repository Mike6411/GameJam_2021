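; Vanishing platform Blueprint that disappears after the first-person character steps into its trigger, then returns.
; The trigger overlap fires a DoOnce that plays the HeatingVelocity timeline, which only serves as a delay here.
; When the timeline finishes, the cube loses collision and is hidden, then both are restored after a short delay.
; The DoOnce is never reset, so the cycle runs only once.
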(event OnComponentBeginOverlap(Trigger)
  (params (OverlappedComponent :type Primitive%20Component%20Object%20Reference) (OtherActor :type Actor%20Object%20Reference) (OtherComp :type Primitive%20Component%20Object%20Reference) (OtherBodyIndex :type Integer) (bFromSweep :type Boolean) (SweepResult :type Hit%20Result%20Structure%20%28by%20ref%29))
  (Utilities|IsValid OtherActor
    (:Is%20Valid
      (Utilities|Casting|CastToFirstPersonCharacter OtherActor)
      (Utilities|FlowControl|DoOnce false
        (:Completed
          (Timeline|Heating%20Velocity PlayFromStart
            (:Finished
              (Collision|SetCollisionEnabled (Variables|Default|GetCube) "NoCollision")
              (Development|SetHiddeninGame (Variables|Default|GetCube) true false)
              (Utilities|FlowControl|Delay 3.0)
              (Collision|SetCollisionEnabled (Variables|Default|GetCube) "QueryAndPhysics")
              (Development|SetHiddeninGame (Variables|Default|GetCube) false false))))))))

(fn ConstructionScript)