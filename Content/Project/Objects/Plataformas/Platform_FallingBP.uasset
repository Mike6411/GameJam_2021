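; Falling platform Blueprint that moves down while the first-person character is inside its box trigger and returns when they leave.
; Overlap begin and end play or reverse the FallPlatform timeline, with play rate derived from Duration.
; The timeline's Fall track lerps MainPlatform's relative location from its BeginPlay position to EndLocation.
; Construction-script nodes for mesh, transform and end-position preview are disconnected and never run.
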(event OnComponentBeginOverlap(BoxCollider)
  (params (OverlappedComponent :type Primitive%20Component%20Object%20Reference) (OtherActor :type Actor%20Object%20Reference) (OtherComp :type Primitive%20Component%20Object%20Reference) (OtherBodyIndex :type Integer) (bFromSweep :type Boolean) (SweepResult :type Hit%20Result%20Structure%20%28by%20ref%29))
  (Utilities|Casting|CastToFirstPersonCharacter OtherActor)
  (Components|Timeline|SetPlayRate (Variables|Default|GetFall%20Platform) (/ 1.0 (Variables|Default|GetDuration)))
  (bind _fall (Timeline|Fall%20Platform Play)
    (:Update
      (Transformation|SetRelativeLocation (Variables|Default|GetMainPlatform) (Math|Vector|Lerp(Vector) (Variables|Default|GetStart_Location) (Variables|Default|GetEnd_Location) _fall) false false))))

(event OnComponentEndOverlap(BoxCollider)
  (params (OverlappedComponent :type Primitive%20Component%20Object%20Reference) (OtherActor :type Actor%20Object%20Reference) (OtherComp :type Primitive%20Component%20Object%20Reference) (OtherBodyIndex :type Integer))
  (Utilities|Casting|CastToFirstPersonCharacter OtherActor)
  (Components|Timeline|SetPlayRate (Variables|Default|GetFall%20Platform) (/ 1.0 (Variables|Default|GetDuration)))
  (bind _fall (Timeline|Fall%20Platform Reverse)
    (:Update
      (Transformation|SetRelativeLocation (Variables|Default|GetMainPlatform) (Math|Vector|Lerp(Vector) (Variables|Default|GetStart_Location) (Variables|Default|GetEnd_Location) _fall) false false))))

(event EventBeginPlay
  (Variables|Default|SetStart_Location (Variables|/Script/Engine.SceneComponent|GetRelativeLocation (Variables|Default|GetMainPlatform))))

(event Collision|EventActorBeginOverlap
  (params (OtherActor :type Actor%20Object%20Reference)))

(event EventTick
  (params (DeltaSeconds :type Float%20%28single-precision%29)))

(fn ConstructionScript)