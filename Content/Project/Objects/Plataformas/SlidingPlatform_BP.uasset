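; Conveyor-style sliding platform that carries the player along its forward direction while they overlap it.
; Each Tick, if the player character overlaps the Eww component, it offsets the character by the platform's forward vector scaled by Speed and delta time, without sweeping.
; The construction script gives Cube a dynamic instance of DubleMaterial_M, deriving its Speed_X parameter from the same Speed so the visual follows the push.
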(event EventTick
  (params (DeltaSeconds :type Float%20%28single-precision%29))
  (bind _returnvalue (Game|GetPlayerCharacter 0))
  (Utilities|IsValid _returnvalue
    (:Is%20Valid
      (if (Collision|IsOverlappingActor (Variables|Default|Geteww) _returnvalue :!class /Script/Engine.PrimitiveComponent)
        (Transformation|AddActorWorldOffset (Game|GetPlayerCharacter 0) (* (Math|Vector|GetForwardVector (Transformation|GetActorRotation)) (* (Utilities|Time|GetWorldDeltaSeconds) (Variables|Default|GetSpeed))))))))

(event EventBeginPlay)

(fn ConstructionScript
  (bind _returnvalue (Rendering|Material|CreateDynamicMaterialInstance "/Game/Materials/DubleMaterial_M.DubleMaterial_M" "None" "None" :!class /Script/Engine.KismetMaterialLibrary))
  (bind _output_get (Variables|Default|SetSliding_M _returnvalue))
  (Rendering|Material|SetMaterial (Variables|Default|GetCube) 0 _output_get)
  (Rendering|Material|SetScalarParameterValue (Variables|Default|GetSliding_M) "Speed_X" (/ (Variables|Default|GetSpeed) -1e+03) :!class /Script/Engine.MaterialInstanceDynamic))