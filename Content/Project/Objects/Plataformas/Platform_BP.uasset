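; Moving platform Blueprint that moves its Platform component between StartPoint and EndPoint.
; On BeginPlay it sets the timeline play rate from PlatformVelocity and starts playback.
; Each timeline update lerps between the two points' current world locations by the Alpha track and sets the platform's world location without sweeping.
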(event EventBeginPlay
  (Components|Timeline|SetPlayRate (Variables|Default|GetPlatform_Movement) (Variables|Default|GetPlatform_Velocity))
  (bind _alpha (Timeline|Platform_Movement Play)
    (:Update
      (Transformation|SetWorldLocation (Variables|Default|GetPlatform) (Math|Vector|Lerp(Vector) (Transformation|GetWorldLocation (Variables|Default|GetStartPoint)) (Transformation|GetWorldLocation (Variables|Default|GetEndPoint)) _alpha) false false))))

(fn ConstructionScript)