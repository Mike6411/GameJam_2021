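; Laser actor that aims a beam at the first-person player and drops a bomb above them.
; Tick attaches the beam particle to Origen once, stores the player's location, then after a random Delay updates the beam end while character movement is active.
; If the player's location matches the stored one, it prints "hit" and spawns a Bomb overhead after another Delay.
; A line trace is left unconnected.
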(event EventBeginPlay)

(event Collision|EventActorBeginOverlap
  (params (OtherActor :type Actor%20Object%20Reference)))

(event EventTick
  (params (DeltaSeconds :type Float%20%28single-precision%29))
  (Utilities|FlowControl|Sequence
    (:then_0
      (Utilities|FlowControl|DoOnce false
        (:Completed
          (bind _returnvalue (Effects|SpawnEmitterAttached "/Game/Project/Material/Laser_particlee.Laser_particlee" (Variables|Default|GetOrigen) "None"))
          (Variables|Default|SetLaser_particles _returnvalue))))
    (:then_1
      (Class|ParticleSystemComponent|SetBeamSourcePoint (Variables|Default|GetLaser_particles) 0 (Transformation|GetWorldLocation (Variables|Default|GetOrigen)))
      (bind _asfirst_person_character (Utilities|Casting|CastToFirstPersonCharacter (Game|GetPlayerCharacter 0)))
      (bind _output_get (Variables|Default|SetTemporal (Transformation|GetActorLocation _asfirst_person_character)))
      (Utilities|FlowControl|Delay (Math|Random|RandomFloatinRange 1.0 2.0))
      (Utilities|FlowControl|Sequence
        (:then_0
          (if (Components|Activation|IsActive (Variables|/Script/Engine.Character|GetCharacterMovement (Game|GetPlayerCharacter 0)))
            (Class|ParticleSystemComponent|SetBeamEndPoint (Variables|Default|GetLaser_particles) 0 (Transformation|GetActorLocation _asfirst_person_character))))
        (:then_1
          (bind _asfirst_person_character_2 (Utilities|Casting|CastToFirstPersonCharacter (Game|GetPlayerCharacter 0)))
          (if (Math|Vector|Equal(Vector) _output_get (Transformation|GetActorLocation _asfirst_person_character_2) 0.0001)
            (Development|PrintString "hit")
            (Utilities|FlowControl|Delay 1.0)
            (Game|SpawnActorfromClass "/Game/Project/Objects/Enemy/Bomb.Bomb_C" (Math|Transform|MakeTransform (Math|Vector|MakeVector (.x (.location (Transformation|GetActorTransform _asfirst_person_character_2))) (.y (.location (Transformation|GetActorTransform _asfirst_person_character_2))) (+ (.z (.location (Transformation|GetActorTransform _asfirst_person_character_2))) 5e+02)) (.rotation (Transformation|GetActorTransform _asfirst_person_character_2)) (.scale (Transformation|GetActorTransform _asfirst_person_character_2))) "AdjustIfPossibleButAlwaysSpawn" 0 0)))))))

(fn ConstructionScript)